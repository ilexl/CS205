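; Grid tile actor for the L_4-Problem level that damages the first-person player on contact when brown.
; The Cube hit event checks for the player character and brown material, then applies one damage.
; A separate ItemSpawner function, not called here, loops over all grid tiles but tests its own Cube for red.
; On a match it spawns a health actor at the iterated tile and restarts the search, with no exit condition.
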(event `self.Cube.OnComponentHit`
  (params (HitComponent :type "PrimitiveComponent Object Reference") (OtherActor :type "Actor Object Reference") (OtherComp :type "PrimitiveComponent Object Reference") (NormalImpulse :type "Vector Structure") (Hit :type "HitResult Structure (by ref)"))
  ;[1 1 1] When player touches Brown platform take 1 Damage
  (bind _asbp_first_person_character (cast `/Game/_TheCubeAssets/Blueprints/Player/Blueprints/BP_FirstPersonCharacter` OtherActor))
  (cast `/Game/_TheCubeAssets/Blueprints/Levels/L_4-Problem/GridTiles_BP` self)
  (if (== (`PrimitiveComponent.GetMaterial` (`self.Cube`) 0) "/Game/_TheCubeAssets/Blueprints/Levels/L_4-Problem/Material_Brown.Material_Brown")
    (`/Game/_TheCubeAssets/Blueprints/Player/Blueprints/BP_FirstPersonCharacter.TakeDamage` _asbp_first_person_character 1.0)))

(fn `ItemSpawner`
  (bind _outactors (`GameplayStatics.GetAllActorsOfClass` "GridTiles_BP_C" :!label _label))
  (for _array_element _outactors
    (if (== (`PrimitiveComponent.GetMaterial` (`self.Cube`) 0) "/Game/_TheCubeAssets/Blueprints/Levels/L_4-Problem/Material_Red.Material_Red")
      (`|SpawnActorFromClass` "/Game/_TheCubeAssets/Blueprints/Items/BP_Health.BP_Health_C" (`KismetMathLibrary.Conv_VectorToTransform` (`self.K2_GetActorLocation` _array_element)) "AdjustIfPossibleButAlwaysSpawn" "MultiplyWithRoot" null null)
      (goto _label))))

(fn `UserConstructionScript`)
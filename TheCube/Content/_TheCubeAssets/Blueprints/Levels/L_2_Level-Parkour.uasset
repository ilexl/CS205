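; Level 2 parkour stage, where lava rises inside glass walls while breakable platforms ride at its height.
; LevelBegin shows the HUD objective and spawns four glass panels below.
; Flag-driven Tick phases lerp the panels up, spawn the lava, then raise it, topping up randomly placed platforms when fewer than five remain.
; Spawns attach to a Blank holder actor, which LevelEnded clears through LevelManager before completing any active objective.
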(event `self.ReceiveBeginPlay`
  (set `self.Level Number` 2))

(event `self.ReceiveTick`
  (params (DeltaSeconds :type "Float (single-precision)"))
  (if (`self.Level In Progress`)
    (if (`self.ToMoveGlassUp`)
      (`self.MovePlatformsUp` DeltaSeconds))
    (if (`self.SpawnLava`)
      (`self.CreateLava`))
    (if (`self.RISE`)
      (`self.RiseLogic` DeltaSeconds))))

(event `/Game/_TheCubeAssets/Blueprints/Levels/I_Level.Level Begin`
  ;[1 0.9369 0] Setup
  (set `self.Level In Progress` true)
  (`KismetSystemLibrary.PrintString` (`KismetStringLibrary.Concat_StrStr` (`KismetStringLibrary.Concat_StrStr` "Level " (`KismetStringLibrary.Conv_IntToString` (`self.Level Number`))) " started!"))
  ;[0 1 0.3254] Show Objective
  (bind _asgi_cube_game_instance (cast `/Game/_TheCubeAssets/Blueprints/GI_CubeGameInstance` (`GameplayStatics.GetGameInstance`)))
  (bind _aswbp_hud (cast `/Game/_TheCubeAssets/UI/WBP_HUD` (`/Game/_TheCubeAssets/Blueprints/GI_CubeGameInstance.HUD Widget` _asgi_cube_game_instance)))
  (`/Game/_TheCubeAssets/UI/WBP_HUD.ShowObjective` _aswbp_hud (+ (`self.Level Number`) 1))
  (`self.GlassPanelsStart`))

(event `/Game/_TheCubeAssets/Blueprints/Levels/I_Level.Spawn Level`
  (params (Transform :type "Transform Structure"))
  (`self.K2_SetActorTransform` Transform false true)
  (set `self.Level In Progress` false))

(fn `CreateLava`
  (bind _returnvalue (`GameplayStatics.GetActorOfClass` "/Game/_TheCubeAssets/Blueprints/Levels/Blank.Blank_C"))
  (bind _returnvalue_2 (`|SpawnActorFromClass` "/Game/_TheCubeAssets/Blueprints/Levels/L_2-Parkour/Lava.Lava_C" (`KismetMathLibrary.MakeTransform` (0.0 0.0 -2000.0)) "AlwaysSpawn" "MultiplyWithRoot" null null))
  (`self.K2_AttachToActor` _returnvalue_2 _returnvalue "None" "KeepWorld" "KeepWorld" "KeepWorld" false)
  (set `self.SpawnLava` false)
  (set `self.RISE` true))

(fn `GetLevelNumber`
  (returns (LevelNumber :type Integer))
  (return (`self.Level Number`)))

(fn `GetRandomPlatformPosition`
  (params (Z :type "Float (double-precision)"))
  (returns (RandomPos :type "Vector Structure"))
  (return (`KismetMathLibrary.MakeVector` (`KismetMathLibrary.RandomFloatInRange` -1200.0 1200.0) (`KismetMathLibrary.RandomFloatInRange` -1200.0 1200.0) Z)))

(fn `GlassPanelsStart`
  (bind _returnvalue (`GameplayStatics.GetActorOfClass` "/Game/_TheCubeAssets/Blueprints/Levels/Blank.Blank_C"))
  (bind _returnvalue_2 (`|SpawnActorFromClass` "/Game/_TheCubeAssets/Blueprints/Levels/L_2-Parkour/GlassWindow.GlassWindow_C" (`KismetMathLibrary.MakeTransform` (0.0 -1750.0 -3800.0)) "AlwaysSpawn" "MultiplyWithRoot" null null))
  (`self.K2_AttachToActor` _returnvalue_2 _returnvalue "None" "KeepWorld" "KeepWorld" "KeepWorld" false)
  (bind _returnvalue_3 (`|SpawnActorFromClass` "/Game/_TheCubeAssets/Blueprints/Levels/L_2-Parkour/GlassWindow.GlassWindow_C" (`KismetMathLibrary.MakeTransform` (0.0 1750.0 -3800.0)) "AlwaysSpawn" "MultiplyWithRoot" null null))
  (`self.K2_AttachToActor` _returnvalue_3 _returnvalue "None" "KeepWorld" "KeepWorld" "KeepWorld" false)
  (bind _returnvalue_4 (`|SpawnActorFromClass` "/Game/_TheCubeAssets/Blueprints/Levels/L_2-Parkour/GlassWindow.GlassWindow_C" (`KismetMathLibrary.MakeTransform` (1750.0 0.0 -3800.0) (struct :`Yaw` 90.0)) "AlwaysSpawn" "MultiplyWithRoot" null null))
  (`self.K2_AttachToActor` _returnvalue_4 _returnvalue "None" "KeepWorld" "KeepWorld" "KeepWorld" false)
  (bind _returnvalue_5 (`|SpawnActorFromClass` "/Game/_TheCubeAssets/Blueprints/Levels/L_2-Parkour/GlassWindow.GlassWindow_C" (`KismetMathLibrary.MakeTransform` (-1750.0 0.0 -3800.0) (struct :`Yaw` 90.0)) "AlwaysSpawn" "MultiplyWithRoot" null null))
  (`self.K2_AttachToActor` _returnvalue_5 _returnvalue "None" "KeepWorld" "KeepWorld" "KeepWorld" false)
  (set `self.ToMoveGlassUp` true))

(fn `Level Ended`
  (bind _returnvalue (`GameplayStatics.GetActorOfClass` "/Game/_TheCubeAssets/Blueprints/LevelManager.LevelManager_C"))
  (`/Game/_TheCubeAssets/Blueprints/LevelManager.Clear Blank Holder` _returnvalue)
  (if (`self.Level In Progress`)
    (`KismetSystemLibrary.PrintString` (`KismetStringLibrary.Concat_StrStr` (`KismetStringLibrary.Concat_StrStr` "Level " (`KismetStringLibrary.Conv_IntToString` (`self.Level Number`))) " ended!"))
    ;[0 1 0.3254] Show Objective
    (bind _asgi_cube_game_instance (cast `/Game/_TheCubeAssets/Blueprints/GI_CubeGameInstance` (`GameplayStatics.GetGameInstance`)))
    (bind _aswbp_hud (cast `/Game/_TheCubeAssets/UI/WBP_HUD` (`/Game/_TheCubeAssets/Blueprints/GI_CubeGameInstance.HUD Widget` _asgi_cube_game_instance)))
    (`/Game/_TheCubeAssets/UI/WBP_HUD.CompleteObjective` _aswbp_hud (+ (`self.Level Number`) 1)))
  (set `self.Level In Progress` false)
  (return))

(fn `MovePlatformsUp`
  (params (DT :type "Float (double-precision)"))
  (bind _outactors (`GameplayStatics.GetAllActorsOfClass` "/Game/_TheCubeAssets/Blueprints/Levels/L_2-Parkour/GlassWindow.GlassWindow_C"))
  (for _array_element _outactors
    (bind _returnvalue (`self.GetTransform` _array_element))
    (bind _location (.location _returnvalue))
    (bind _returnvalue_2 (`KismetMathLibrary.MakeVector` (.x _location) (.y _location) -240.0))
    (bind _returnvalue_3 (`KismetMathLibrary.MakeTransform` _returnvalue_2 (.rotation _returnvalue) (.scale _returnvalue)))
    (`self.K2_SetActorTransform` _array_element (`KismetMathLibrary.TLerp` _returnvalue _returnvalue_3 DT) false true)
    (if (<= (`KismetMathLibrary.Vector_Distance` _location _returnvalue_2) 0.1)
      (`self.K2_SetActorTransform` _array_element _returnvalue_3 false true)
      (set `self.ToMoveGlassUp` false)))
  (if (not (`self.ToMoveGlassUp`))
    (set `self.SpawnLava` true)))

(fn `RiseLogic`
  (params (DT :type "Float (double-precision)"))
  (bind _returnvalue (`GameplayStatics.GetActorOfClass` "/Game/_TheCubeAssets/Blueprints/Levels/L_2-Parkour/Lava.Lava_C"))
  (bind _returnvalue_2 (`KismetMathLibrary.TLerp` (`self.GetTransform` _returnvalue) (`KismetMathLibrary.MakeTransform` (0.0 0.0 -250.0)) (* DT (`self.RiseRate`))))
  (`self.K2_SetActorTransform` _returnvalue _returnvalue_2 false false)
  (bind _outactors (`GameplayStatics.GetAllActorsOfClass` "/Game/_TheCubeAssets/Blueprints/Levels/L_2-Parkour/BreakablePlatform.BreakablePlatform_C"))
  (for _array_element _outactors
    (bind _z (.z (.location _returnvalue_2)))
    (`self.K2_SetActorTransform` _array_element (`KismetMathLibrary.MakeTransform` (`KismetMathLibrary.MakeVector` (.x (.location (`self.GetTransform` _array_element))) (.y (.location (`self.GetTransform` _array_element))) _z) (.rotation (`self.GetTransform` _array_element)) (.scale (`self.GetTransform` _array_element))) false false))
  (if (< (`KismetArrayLibrary.Array_Length` _outactors) 5)
    (bind _returnvalue_3 (`GameplayStatics.GetActorOfClass` "/Game/_TheCubeAssets/Blueprints/Levels/Blank.Blank_C"))
    (bind _randompos (`self.GetRandomPlatformPosition` _z))
    (bind _returnvalue_4 (`|SpawnActorFromClass` "/Game/_TheCubeAssets/Blueprints/Levels/L_2-Parkour/BreakablePlatform.BreakablePlatform_C" (`KismetMathLibrary.MakeTransform` _randompos) "AlwaysSpawn" "MultiplyWithRoot" null null))
    (`self.K2_AttachToActor` _returnvalue_4 _returnvalue_3 "None" "KeepWorld" "KeepWorld" "KeepWorld" false)))

(fn `UserConstructionScript`)
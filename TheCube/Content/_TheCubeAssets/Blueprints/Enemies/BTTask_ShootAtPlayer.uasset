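; Behavior Tree task that makes a ranged, flying ranged or boss enemy perform its attack.
; On AI execution it casts the controlled pawn to Ranged_Enemy, then FlyingRanged_Enemy, then BOSS_Enemy, and calls Attack on the first match.
; After a brief delay, shorter for the boss, it finishes the task with the attack's result.
; Any other pawn type leaves the task without a finish call.
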(event `self.ReceiveExecuteAI`
  (params (OwnerController :type "AIController Object Reference") (ControlledPawn :type "Pawn Object Reference"))
  (bind _asranged_enemy (cast `/Game/_TheCubeAssets/Blueprints/Enemies/Ranged_Enemy` ControlledPawn)
    (:`then`
      (bind _fired (`/Game/_TheCubeAssets/Blueprints/Enemies/Ranged_Enemy.Attack` _asranged_enemy))
      (`KismetSystemLibrary.Delay` 0.1)
      (`self.FinishExecute` _fired))
    (:`CastFailed`
      (bind _asflying_ranged_enemy (cast `/Game/_TheCubeAssets/Blueprints/Enemies/FlyingRanged_Enemy` ControlledPawn)
        (:`then`
          (bind _fired_2 (`/Game/_TheCubeAssets/Blueprints/Enemies/FlyingRanged_Enemy.Attack` _asflying_ranged_enemy))
          (`KismetSystemLibrary.Delay` 0.1)
          (`self.FinishExecute` _fired_2))
        (:`CastFailed`
          (bind _asboss_enemy (cast `/Game/_TheCubeAssets/Blueprints/Enemies/BOSS_Enemy` ControlledPawn))
          (bind _fired_3 (`/Game/_TheCubeAssets/Blueprints/Enemies/BOSS_Enemy.Attack` _asboss_enemy))
          (`KismetSystemLibrary.Delay` 0.001)
          (`self.FinishExecute` _fired_3))))))
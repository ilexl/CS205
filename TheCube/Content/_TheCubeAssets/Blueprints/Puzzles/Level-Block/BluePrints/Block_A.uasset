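; Block_A is a puzzle block actor that travels along a spline path when its MoveObject event is triggered.
; On BeginPlay it caches the first SplinePath_BP actor found in the level.
; MoveObject plays a timeline scaled by TimeToComplete, setting the block's location and rotation by distance along the spline.
; The spline is sampled in local space but applied as the actor's world transform.
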(event `self.ReceiveBeginPlay`
  (bind _returnvalue (`GameplayStatics.GetActorOfClass` "/Game/_TheCubeAssets/Blueprints/Puzzles/Level-Block/BluePrints/SplinePath_BP.SplinePath_BP_C"))
  (set `self.Spline REF` _returnvalue))

(event `Move Object`
  (bind _spline (`/Game/_TheCubeAssets/Blueprints/Puzzles/Level-Block/BluePrints/SplinePath_BP.Spline` (`self.Spline REF`)))
  (`TimelineComponent.SetPlayRate` (`self.Move Object T`) (/ 1.0 (`self.TimeToComplete`)))
  (bind (_direction _move_track) (`Timeline|Move Object T`)
    (:`Update`
      (bind _returnvalue (`KismetMathLibrary.Lerp` 0.0 (`SplineComponent.GetSplineLength` (`/Game/_TheCubeAssets/Blueprints/Puzzles/Level-Block/BluePrints/SplinePath_BP.Spline` (`self.Spline REF`))) _move_track))
      (`self.K2_SetActorTransform` (`KismetMathLibrary.MakeTransform` (`SplineComponent.GetLocationAtDistanceAlongSpline` _spline _returnvalue "Local") (`SplineComponent.GetRotationAtDistanceAlongSpline` _spline _returnvalue "Local"))))))

(fn `UserConstructionScript`)
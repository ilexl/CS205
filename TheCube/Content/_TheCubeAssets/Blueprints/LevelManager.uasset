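; Level manager actor that builds the game's six levels as the faces of a cube around itself.
; On BeginPlay it computes a transform for each side and spawns the maze, waves, parkour, cubes, problem and boss levels.
; Through the I_Level interface, it places each level on its side, deactivates it and attaches it to the manager.
; A debug flag, forced on at startup, prints each level's placement.
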(event `self.ReceiveBeginPlay`
  (bind _sidetransforms (`self.SideTransforms`))
  ;[0 0 0] Initilize
  ;;[0.1354 1 0] 100 * scale of base * 0.5
  (set `self.Level Depth` 2000.0)
  (`KismetArrayLibrary.Array_Add` _sidetransforms (`KismetMathLibrary.MakeTransform` (`KismetMathLibrary.MakeVector` 0.0 0.0 (`self.Level Depth`))))
  (`KismetArrayLibrary.Array_Add` _sidetransforms (`KismetMathLibrary.MakeTransform` (`KismetMathLibrary.MakeVector` 0.0 (`self.Level Depth`)) (struct :`Roll` 90.0)))
  (`KismetArrayLibrary.Array_Add` _sidetransforms (`KismetMathLibrary.MakeTransform` (`KismetMathLibrary.MakeVector` (`self.Level Depth`)) (struct :`Pitch` 90.0)))
  (`KismetArrayLibrary.Array_Add` _sidetransforms (`KismetMathLibrary.MakeTransform` (`KismetMathLibrary.MakeVector` (* (`self.Level Depth`) -1.0)) (struct :`Pitch` 270.0)))
  (`KismetArrayLibrary.Array_Add` _sidetransforms (`KismetMathLibrary.MakeTransform` (`KismetMathLibrary.MakeVector` 0.0 (* (`self.Level Depth`) -1.0)) (struct :`Roll` 270.0)))
  (`KismetArrayLibrary.Array_Add` _sidetransforms (`KismetMathLibrary.MakeTransform` (`KismetMathLibrary.MakeVector` 0.0 0.0 (* (`self.Level Depth`) -1.0)) (struct :`Roll` 180.0)))
  ;;[1 0 0.8051] DEBUG ONLY
  (set `self.DEBUG` true)
  ;;[0.9964 1 0.5167] Create Levels
  (bind _returnvalue (`|SpawnActorFromClass` "/Game/_TheCubeAssets/Blueprints/Levels/L_0_Level-Maze.L_0_Level-Maze_C" (`self.TransformBLANK`) "Undefined" "MultiplyWithRoot" null null))
  (bind _asi_level (cast `/Game/_TheCubeAssets/Blueprints/I_Level` _returnvalue))
  (`KismetArrayLibrary.Array_Add` (`self.LevelsInterface`) _asi_level)
  (bind _returnvalue_2 (`|SpawnActorFromClass` "/Game/_TheCubeAssets/Blueprints/Levels/L_1_Level-Waves.L_1_Level-Waves_C" (`self.TransformBLANK`) "Undefined" "MultiplyWithRoot" null null))
  (bind _asi_level_2 (cast `/Game/_TheCubeAssets/Blueprints/I_Level` _returnvalue_2))
  (`KismetArrayLibrary.Array_Add` (`self.LevelsInterface`) _asi_level_2)
  (bind _returnvalue_3 (`|SpawnActorFromClass` "/Game/_TheCubeAssets/Blueprints/Levels/L_2_Level-Parkour.L_2_Level-Parkour_C" (`self.TransformBLANK`) "Undefined" "MultiplyWithRoot" null null))
  (bind _asi_level_3 (cast `/Game/_TheCubeAssets/Blueprints/I_Level` _returnvalue_3))
  (`KismetArrayLibrary.Array_Add` (`self.LevelsInterface`) _asi_level_3)
  (bind _returnvalue_4 (`|SpawnActorFromClass` "/Game/_TheCubeAssets/Blueprints/Levels/L_3_Level-Cubes.L_3_Level-Cubes_C" (`self.TransformBLANK`) "Undefined" "MultiplyWithRoot" null null))
  (bind _asi_level_4 (cast `/Game/_TheCubeAssets/Blueprints/I_Level` _returnvalue_4))
  (`KismetArrayLibrary.Array_Add` (`self.LevelsInterface`) _asi_level_4)
  (bind _returnvalue_5 (`|SpawnActorFromClass` "/Game/_TheCubeAssets/Blueprints/Levels/L_4_Level-Problem.L_4_Level-Problem_C" (`self.TransformBLANK`) "Undefined" "MultiplyWithRoot" null null))
  (bind _asi_level_5 (cast `/Game/_TheCubeAssets/Blueprints/I_Level` _returnvalue_5))
  (`KismetArrayLibrary.Array_Add` (`self.LevelsInterface`) _asi_level_5)
  (bind _returnvalue_6 (`|SpawnActorFromClass` "/Game/_TheCubeAssets/Blueprints/Levels/L_5_Level-Boss.L_5_Level-Boss_C" (`self.TransformBLANK`) "Undefined" "MultiplyWithRoot" null null))
  (bind _asi_level_6 (cast `/Game/_TheCubeAssets/Blueprints/I_Level` _returnvalue_6))
  (`KismetArrayLibrary.Array_Add` (`self.LevelsInterface`) _asi_level_6)
  ;;[0 0.05366 1] Move all transforms and Deactive
  (for (_array_element _array_index) (`self.LevelsInterface`)
    (if (`self.DEBUG`)
      ;;;[1 0 0.8051] DEBUG
      (`KismetSystemLibrary.PrintString` (`KismetStringLibrary.Concat_StrStr` (`KismetStringLibrary.Concat_StrStr` (`KismetStringLibrary.Concat_StrStr` "Initialized Level " (`KismetStringLibrary.Conv_IntToString` _array_index)) " @ transform ") (`KismetStringLibrary.Conv_TransformToString` (`|GetArrayItem` (`self.SideTransforms`) _array_index)))))
    (`/Game/_TheCubeAssets/Blueprints/I_Level.Spawn Level` _array_element (`|GetArrayItem` (`self.SideTransforms`) _array_index))
    (`/Game/_TheCubeAssets/Blueprints/I_Level.SetActive` _array_element false)
    (bind _asactor (cast `Actor` (`KismetSystemLibrary.Conv_InterfaceToObject` _array_element))
      (:`then`
        (`self.K2_AttachToActor` _asactor self "None" "KeepRelative" "KeepRelative" "KeepRelative" true))
      (:`CastFailed`
        (`KismetSystemLibrary.PrintString` "Error: Unable to cast target to actor #876")))))

(fn `UserConstructionScript`)
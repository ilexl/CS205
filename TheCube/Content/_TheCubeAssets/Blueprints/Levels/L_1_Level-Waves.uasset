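; Level 1 wave controller actor that tracks whether the level is in progress and announces its start and end.
; SpawnLevel teleports the actor to a given transform and clears the in-progress flag.
; LevelBegin sets the flag, prints a start message and spawns a single TestEnemy at a fixed location; LevelEnded clears the flag, printing only if it was running.
; Tick checks the flag but has no logic yet.
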(event `self.ReceiveBeginPlay`
  (set `self.Level Number` 1))

(event `self.ReceiveTick`
  (params (DeltaSeconds :type "Float (single-precision)"))
  (if (`self.Level In Progress`)
    _))

(event `/Game/_TheCubeAssets/Blueprints/Levels/I_Level.Spawn Level`
  (params (Transform :type "Transform Structure"))
  (`self.K2_SetActorTransform` Transform false true)
  (set `self.Level In Progress` false))

(event `/Game/_TheCubeAssets/Blueprints/Levels/I_Level.Level Begin`
  (set `self.Level In Progress` true)
  (`KismetSystemLibrary.PrintString` (`KismetStringLibrary.Concat_StrStr` (`KismetStringLibrary.Concat_StrStr` "Level " (`KismetStringLibrary.Conv_IntToString` (`self.Level Number`))) " started!"))
  (`|SpawnActorFromClass` "/Game/_TheCubeAssets/Blueprints/Enemies/Test-Enemy.Test-Enemy_C" (`KismetMathLibrary.MakeTransform` (0.0 0.0 -1000.0)) "AdjustIfPossibleButAlwaysSpawn" "MultiplyWithRoot" null null))

(fn `GetLevelNumber`
  (returns (LevelNumber :type Integer))
  (return (`self.Level Number`)))

(fn `Level Ended`
  (if (`self.Level In Progress`)
    (`KismetSystemLibrary.PrintString` (`KismetStringLibrary.Concat_StrStr` (`KismetStringLibrary.Concat_StrStr` "Level " (`KismetStringLibrary.Conv_IntToString` (`self.Level Number`))) " ended!")))
  (set `self.Level In Progress` false)
  (return))

(fn `UserConstructionScript`)
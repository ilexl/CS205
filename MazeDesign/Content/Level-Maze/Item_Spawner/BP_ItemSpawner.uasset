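; BP_ItemSpawner populates the maze's end tiles with random items when play begins.
; On BeginPlay, AttemptToSpawn calls SpawnItem unless CurrentItem is still valid.
; SpawnItem reads the EndMazeTile transforms from the first BP_Maze found and spawns a random ItemsToSpawn class at each, adjusting for collision but always spawning.
; CurrentItem is overwritten on each spawn, so it tracks only the last item.
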(event `self.ReceiveBeginPlay`
  (`self.AttemptToSpawn`))

(fn `AttemptToSpawn`
  ;[1 1 1] Checks if Item is there and if not Calls Spawn Item Function
  (`/Engine/EditorBlueprintResources/StandardMacros.IsValid` (`self.CurrentItem`)
    (:`Is Valid`
      (`KismetSystemLibrary.PrintString` "Item already spawned"))
    (:`Is Not Valid`
      (`self.SpawnItem`))))

(fn `SpawnItem`
  ;[1 1 1] Gets all Actors of BP Maze, targets End Maze Tiles Loops through them
  (bind _outactors (`GameplayStatics.GetAllActorsOfClass` "/Game/Level-Maze/Blueprints/BP_Maze.BP_Maze_C"))
  (for _array_element (`/Game/Level-Maze/Blueprints/BP_Maze.EndMazeTile` (`|GetArrayItem` _outactors))
    ;[1 1 1] Spawns Items at End Maze Tiles location
    (bind _returnvalue (`|SpawnActorFromClass` (`|GetArrayItem` (`self.ItemsToSpawn`) (`KismetMathLibrary.RandomIntegerInRange` 0 (- (`KismetArrayLibrary.Array_Length` (`self.ItemsToSpawn`)) 1))) _array_element "AdjustIfPossibleButAlwaysSpawn" "MultiplyWithRoot" null null))
    (set `self.CurrentItem` _returnvalue)))

(fn `UserConstructionScript`)
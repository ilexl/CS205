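; Lava hazard volume that damages the first-person player while they stand in it.
; On overlap, it applies damage and spawns an explosion particle and sound at the player's location.
; A one-second Delay loops this sequence while an InLava flag stays true, and end overlap from any actor clears the flag.
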(event `self.LavaVol.OnComponentBeginOverlap`
  (params (OverlappedComponent :type "PrimitiveComponent Object Reference") (OtherActor :type "Actor Object Reference") (OtherComp :type "PrimitiveComponent Object Reference") (OtherBodyIndex :type Integer) (bFromSweep :type Boolean) (SweepResult :type "HitResult Structure (by ref)"))
  ;[1 1 1] When Player enters Lava Take damage then loops after 1 second delay, also makes sound and explosion animation
  (set `self.InLava` true)
  (bind _asbp_first_person_character (cast `/Game/_TheCubeAssets/Blueprints/Player/Blueprints/BP_FirstPersonCharacter` OtherActor :!label _label))
  (`/Game/_TheCubeAssets/Blueprints/Player/Blueprints/BP_FirstPersonCharacter.TakeDamage` _asbp_first_person_character 5.0)
  (bind _returnvalue (`self.K2_GetActorLocation` _asbp_first_person_character))
  (`GameplayStatics.SpawnEmitterAtLocation` "/Game/StarterContent/Particles/P_Explosion.P_Explosion" _returnvalue)
  (`GameplayStatics.SpawnSoundAtLocation` "/Game/StarterContent/Audio/Explosion01.Explosion01" _returnvalue (struct) 1.0 1.0 0.0 null null)
  (`KismetSystemLibrary.Delay` 1.0)
  (if (`self.InLava`)
    (goto _label)))

(event `self.LavaVol.OnComponentEndOverlap`
  (params (OverlappedComponent :type "PrimitiveComponent Object Reference") (OtherActor :type "Actor Object Reference") (OtherComp :type "PrimitiveComponent Object Reference") (OtherBodyIndex :type Integer))
  ;[1 1 1] When Player enters Lava Take damage then loops after 1 second delay, also makes sound and explosion animation
  (set `self.InLava` false))

(fn `UserConstructionScript`)
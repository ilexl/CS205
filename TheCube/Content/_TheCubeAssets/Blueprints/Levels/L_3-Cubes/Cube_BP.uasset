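; Cube actor that travels along a spline path placed in the level when play begins.
; BeginPlay finds the SplinePath_BP actor and starts a timeline whose play rate derives from TimeToComplete.
; Each timeline update maps the track alpha to a distance along the spline and sets the cube's world location and rotation from that point.
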(event `self.ReceiveBeginPlay`
  ;[1 1 1] Plays, tells cube to move along Spline path actor
  (bind _returnvalue (`GameplayStatics.GetActorOfClass` "/Game/_TheCubeAssets/Blueprints/Levels/L_3-Cubes/SplinePath_BP.SplinePath_BP_C"))
  (set `self.SplineREF` _returnvalue)
  (`self.Move Object`))

(event `Move Object`
  (bind _spline (`/Game/_TheCubeAssets/Blueprints/Levels/L_3-Cubes/SplinePath_BP.Spline` (`self.SplineREF`)))
  ;[1 1 1] When played sets play rate to .2 secs to move object
  (`TimelineComponent.SetPlayRate` (`self.MoveObjectT`) (/ 1.0 (`self.Time To Complete`)))
  ;[1 1 1] Starts Timeline
  (bind (_direction _movetrack) (`Timeline|MoveObjectT`)
    (:`Update`
      (bind _returnvalue (`KismetMathLibrary.Lerp` 0.0 (`SplineComponent.GetSplineLength` (`/Game/_TheCubeAssets/Blueprints/Levels/L_3-Cubes/SplinePath_BP.Spline` (`self.SplineREF`))) _movetrack))
      (`self.K2_SetActorTransform` (`KismetMathLibrary.MakeTransform` (`SplineComponent.GetLocationAtDistanceAlongSpline` _spline _returnvalue "World") (`SplineComponent.GetRotationAtDistanceAlongSpline` _spline _returnvalue "World"))))))

(fn `UserConstructionScript`)
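; FlyingRanged_Enemy is a flying ranged enemy Blueprint, built on a parent class, with an attack that is still a placeholder.
; Construction fills its health to maximum, and BeginPlay sets the reload time and lifts the Cube and Widget components to a hover height.
; Tick accumulates time since the last shot, which gates Attack.
; When ready, Attack only prints a not-implemented message, resets the timer and reports success.
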(event `self.ReceiveBeginPlay`
  (`parent.ReceiveBeginPlay`)
  (set `self.ReloadTime` 5.0)
  (set `self.TimeSinceLastShot` 0.0)
  (set `self.OffsetZ` (0.0 0.0 200.0))
  (`SceneComponent.K2_AddLocalOffset` (`self.Widget`) (`self.OffsetZ`) false true)
  (`SceneComponent.K2_AddLocalOffset` (`self.Cube`) (`self.OffsetZ`) false true))

(event `self.ReceiveTick`
  (params (DeltaSeconds :type "Float (single-precision)"))
  (`parent.ReceiveTick` DeltaSeconds)
  (set `self.TimeSinceLastShot` (+ DeltaSeconds (`self.TimeSinceLastShot`))))

(fn `Attack`
  (returns (Fired :type Boolean))
  (if (> (`self.TimeSinceLastShot`) (`self.ReloadTime`))
    (`KismetSystemLibrary.PrintString` "Attack Needs Implementing")
    (set `self.TimeSinceLastShot` 0.0)
    (return true)
    (else
      (return false))))

(fn `UserConstructionScript`
  (bind _output_get (set `self.MaxHealth` 100.0))
  (set `self.Health` _output_get)
  (`parent.UserConstructionScript`))
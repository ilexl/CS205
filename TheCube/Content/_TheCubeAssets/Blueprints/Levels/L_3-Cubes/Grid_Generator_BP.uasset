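; Grid generator Blueprint that lays out copies of a static mesh in a square grid for level building.
; The Construction Script adds GridSize squared mesh components, using X and Y counters to wrap to a new row after GridSize entries.
; Each component is offset by the mesh's local bounds size, with DistanceX and DistanceY adding gaps as multiples of that size.
; BeginPlay is empty.
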(event `self.ReceiveBeginPlay`)

(fn `UserConstructionScript`
  (bind _grid_size (`self.grid size`))
  (bind _x_coord (`self.X Coord`))
  (bind _y_coord (`self.Y Coord`))
  ;[1 1 1] Grid Size starts index 1
  (for _ (range 1 (+ (* _grid_size _grid_size) 1))
    ;[1 1 1] If X Coord is less than Grid size create mesh otherwise return to 0 for Y Coord
    (if (> (`self.X Coord`) (- (`self.grid size`) 1)) :!label _label
      (set `self.X Coord` 0)
      (bind _result (`/Engine/EditorBlueprintResources/StandardMacros.IncrementInt` (`self.Y Coord`))
        (:`  `
          (set `self.Y Coord` _result)
          (goto _label)))
      (else
        (bind _returnvalue (`AddComponent|NODE_AddStaticMeshComponent-0`))
        ;[1 1 1] Sets location of static meshes
        (`StaticMeshComponent.SetStaticMesh` _returnvalue (`self.grid mesh`))
        (bind (_min _max) (`StaticMeshComponent.GetLocalBounds` _returnvalue))
        (bind (_returnvalue_x _returnvalue_y) (`KismetMathLibrary.BreakVector` (- _max _min)))
        (`SceneComponent.K2_SetRelativeLocation` _returnvalue (`KismetMathLibrary.MakeVector` (+ (* _returnvalue_x _x_coord) (* _returnvalue_x _x_coord (`self.distance_X`))) (+ (* _y_coord _returnvalue_y (`self.distance_Y`)) (* _returnvalue_y _y_coord))) false false)
        (bind _result_2 (`/Engine/EditorBlueprintResources/StandardMacros.IncrementInt` (`self.X Coord`))
          (:`  `
            (set `self.X Coord` _result_2)))))))
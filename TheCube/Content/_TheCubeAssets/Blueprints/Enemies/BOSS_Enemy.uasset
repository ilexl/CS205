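; BOSS_Enemy is a high-health boss enemy that attacks by firing oversized projectiles, building on a parent class's logic.
; The construction script sets its maximum and current health before running the parent's construction script.
; Tick accumulates time since the last shot, gating Attack behind a reload cooldown.
; Attack spawns a scaled-up BP_EnemyProjectile at ShootLocation, resets the timer and returns whether it fired.
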(event `self.ReceiveBeginPlay`
  (`parent.ReceiveBeginPlay`)
  (set `self.ReloadTime` 5.0)
  (set `self.TimeSinceLastShot` 0.0))

(event `self.ReceiveTick`
  (params (DeltaSeconds :type "Float (single-precision)"))
  (`parent.ReceiveTick` DeltaSeconds)
  (set `self.TimeSinceLastShot` (+ DeltaSeconds (`self.TimeSinceLastShot`))))

(fn `Attack`
  (returns (Fired :type Boolean))
  (if (> (`self.TimeSinceLastShot`) (`self.ReloadTime`))
    (`|SpawnActorFromClass` "/Game/_TheCubeAssets/Blueprints/Enemies/BP_EnemyProjectile.BP_EnemyProjectile_C" (`KismetMathLibrary.MakeTransform` (.location (`SceneComponent.K2_GetComponentToWorld` (`self.Shoot Location`))) (.rotation (`SceneComponent.K2_GetComponentToWorld` (`self.Shoot Location`))) (10.0 10.0 10.0)) "Undefined" "MultiplyWithRoot" null null)
    (set `self.TimeSinceLastShot` 0.0)
    (return true)
    (else
      (return false))))

(fn `UserConstructionScript`
  (bind _output_get (set `self.MaxHealth` 1000.0))
  (set `self.Health` _output_get)
  (`parent.UserConstructionScript`))
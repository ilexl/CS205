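; Instance manager Blueprint, filed under the Maze level puzzles, that adds and clears static mesh instances.
; A map holds one Hierarchical Instanced Static Mesh component per mesh, created on first use by AddNewMeshInstance, which returns the new instance index and prints a debug string.
; Removal functions clear all instances, clear one mesh's instances, or remove a single instance, though the latter ignores its Index input and always removes instance 0.
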(fn `AddNewMeshInstance`
  (params (Mesh :type "StaticMesh Object Reference") (Transform :type "Transform Structure"))
  (returns (`Successful?` :type Boolean) (Index :type Integer))
  (bind (_value _returnvalue) (`BlueprintMapLibrary.Map_Find` (`self.InstanceComponentList`) Mesh))
  (`KismetSystemLibrary.PrintString` "Hello")
  (if _returnvalue
    (bind _returnvalue_2 (`InstancedStaticMeshComponent.AddInstance` _value Transform false))
    (return true _returnvalue_2)
    (else
      (bind _returnvalue_3 (`AddComponent|NODE_AddHierarchicalInstancedStaticMeshComponent-2`))
      (`BlueprintMapLibrary.Map_Add` (`self.InstanceComponentList`) Mesh _returnvalue_3)
      (`StaticMeshComponent.SetStaticMesh` _returnvalue_3 Mesh)
      (bind _returnvalue_4 (`InstancedStaticMeshComponent.AddInstance` _returnvalue_3 Transform false))
      (return true _returnvalue_4))))

(fn `RemoveAllinstances`
  (returns (`Succesful?` :type Boolean))
  (bind _keys (`BlueprintMapLibrary.Map_Keys` (`self.InstanceComponentList`)))
  (for _array_element _keys
    (`InstancedStaticMeshComponent.ClearInstances` (`BlueprintMapLibrary.Map_Find` (`self.InstanceComponentList`) _array_element)))
  (return true))

(fn `RemoveAllMeshInstances`
  (params (Mesh :type "StaticMesh Object Reference"))
  (returns (`Succesful?` :type Boolean))
  (bind (_value _returnvalue) (`BlueprintMapLibrary.Map_Find` (`self.InstanceComponentList`) Mesh))
  (if _returnvalue
    (`InstancedStaticMeshComponent.ClearInstances` _value)
    (return true)
    (else
      (return true))))

(fn `RemoveMeshInstance`
  (params (Mesh :type "StaticMesh Object Reference") (Index :type Integer))
  (returns (`Succesful?` :type Boolean))
  (bind (_value _returnvalue) (`BlueprintMapLibrary.Map_Find` (`self.InstanceComponentList`) Mesh))
  (if _returnvalue
    (bind _returnvalue_2 (`InstancedStaticMeshComponent.RemoveInstance` _value 0))
    (return _returnvalue_2)
    (else
      (return false))))

(fn `UserConstructionScript`)
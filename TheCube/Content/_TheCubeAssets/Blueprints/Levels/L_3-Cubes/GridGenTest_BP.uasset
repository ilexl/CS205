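; GridGenTest_BP is a test grid generator that spawns a flat grid of GridTile_BP actors from its own location at BeginPlay.
; A single loop up to MaxActors converts each index to a cell by dividing by MaxRows, with the remainder setting X and the whole quotient setting Y.
; Both offsets are scaled by ActorSpacing, and the construction script is empty.
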(event `self.ReceiveBeginPlay`
  (bind (_returnvalue_x _returnvalue_y) (`KismetMathLibrary.BreakVector` (`self.K2_GetActorLocation`)))
  (bind _actorspacing (`self.ActorSpacing`))
  (for _index (range (+ (`self.MaxActors`) 1))
    (bind (_remainder _returnvalue) (`KismetMathLibrary.FMod` (`KismetMathLibrary.Conv_IntToDouble` _index) (`self.MaxRows`)))
    (`|SpawnActorFromClass` "/Game/_TheCubeAssets/Blueprints/Levels/L_3-Cubes/GridTile_BP.GridTile_BP_C" (`KismetMathLibrary.MakeTransform` (`KismetMathLibrary.MakeVector` (+ (* _remainder _actorspacing) _returnvalue_x) (+ (* _returnvalue _actorspacing) _returnvalue_y))) "Undefined" "MultiplyWithRoot" null null)))

(fn `UserConstructionScript`)